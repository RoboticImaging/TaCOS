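; CharacterBP is a first-person character Blueprint with a configurable camera and scene capture, and it resets global time dilation on BeginPlay.
; SetCam applies pitch, focal length, sensor size and horizontal resolution, setting focal length on the first-person camera and resolution on the CineCaptureComponent2D render target.
; Activate and deactivate functions toggle character movement and the stop state of the AutoAgent actor found in the level.
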(event `self.ReceiveBeginPlay`
  (`GameplayStatics.SetGlobalTimeDilation` 1.0))

(fn `ActivateCharacter`
  (`ActorComponent.Activate` (`self.CharacterMovement`) false)
  (bind _returnvalue (`GameplayStatics.GetActorOfClass` "/Script/ProceduralGeneration.AutoAgent"))
  (`AutoAgent.SetStop` _returnvalue false))

(fn `Deactivate Character`
  (`ActorComponent.Deactivate` (`self.CharacterMovement`))
  (bind _returnvalue (`GameplayStatics.GetActorOfClass` "/Script/ProceduralGeneration.AutoAgent"))
  (`AutoAgent.SetStop` _returnvalue true))

(fn `Set Cam`
  (params (Pitch :type "Float (double-precision)") (FL :type "Float (double-precision)") (`Sensor Width` :type "Float (double-precision)") (`Sensor Height` :type "Float (double-precision)") (ResX :type Integer))
  (`self.ChangeOrientation` Pitch)
  (`self.Set FL` FL)
  (`self.Set ResX` ResX)
  (`self.ChangeSensorSize` `Sensor Width` `Sensor Height`))

(fn `Set FL`
  (params (`Focal Length` :type "Float (double-precision)"))
  (set `CineCameraComponent.CurrentFocalLength` `Focal Length` (`self.FirstPersonCameraComponent`)))

(fn `Set ResX`
  (params (`Res X` :type Integer))
  (set `CineCaptureComponent2D.RenderTargetHighestDimension` `Res X` (`self.CineCaptureComponent2D`)))

(fn `UserConstructionScript`)