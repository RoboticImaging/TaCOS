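; TCP client that lets a local external process run camera-configuration trials and capture synthetic training images.
; Each comma-separated message sets CharacterBP's orientation, lens, sensor, resolution and a solution number, then restarts character and AutoAgent movement.
; A delayed-loop macro exports the CharacterView render target, saving frames as training images when ProceduralRoom finds a bounding box, otherwise as feature images.
; On completion it stops movement and sends threshold counts back over the socket.
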(event `self.ReceiveBeginPlay`
  (bind _connectionid (`self.Connect` "127.0.0.1" 3457 (delegate `Disconnected`) (delegate `Connected`) (delegate `ReceivedMessage`)))
  (set `self.Connection ID` _connectionid)
  (set `self.Path` "E:\\train_data"))

(event `Disconnected`
  (params (ConnectionId :type Integer)))

(event `Connected`
  (params (ConnectionId :type Integer))
  (if true
    (`KismetSystemLibrary.PrintString` "Connected")))

(event `ReceivedMessage`
  (params (ConnectionId :type Integer) (Message :type "Array of Byte (by ref)"))
  (`KismetSystemLibrary.PrintString` "Received!")
  (bind _returnvalue (`self.Message_ReadString` Message (`KismetArrayLibrary.Array_Length` Message)))
  (bind _returnvalue_2 (`KismetStringLibrary.ParseIntoArray` _returnvalue ","))
  (`self.Set Orientation` (`KismetStringLibrary.Conv_StringToDouble` (`|GetArrayItem` _returnvalue_2)))
  (`self.Set Focal Length` (`KismetStringLibrary.Conv_StringToDouble` (`|GetArrayItem` _returnvalue_2 1)))
  (bind _returnvalue_3 (`KismetStringLibrary.Conv_StringToInt` (`|GetArrayItem` _returnvalue_2 4)))
  (`self.SetResolution` _returnvalue_3)
  (`KismetSystemLibrary.Delay` 0.2)
  (`self.Set Sensor Size` (`KismetStringLibrary.Conv_StringToDouble` (`|GetArrayItem` _returnvalue_2 2)) (`KismetStringLibrary.Conv_StringToDouble` (`|GetArrayItem` _returnvalue_2 3)))
  (set `self.SolutionNo` (`KismetStringLibrary.Conv_StringToInt` (`|GetArrayItem` _returnvalue_2 6)))
  (`KismetSystemLibrary.Delay` 2.0)
  (`self.ResetThresholdCount`)
  (`self.ResumeMovement`)
  (`self.ResumeToTargets`)
  (set `self.train_idx` 0)
  (`self.Set Feature Image Path` 0 (`self.SolutionNo`))
  (bind _index (`self.For Loop with Delay` 0 500 0.3)
    (:`Loop Body`
      (bind _ifboundingbox (`self.GetBoundingBox` (`self.SolutionNo`) (`self.train_idx`) _returnvalue_3 (`KismetStringLibrary.Conv_StringToInt` (`|GetArrayItem` _returnvalue_2 5))))
      (if _ifboundingbox
        (bind (_path _name) (`self.Set Train Image Path` (`self.train_idx`) (`self.SolutionNo`)))
        (`self.ExportRender` _path _name)
        (`self.CopyImageToPath` (`self.SolutionNo`) _index (`self.train_idx`))
        (set `self.train_idx` (+ (`self.train_idx`) 1))
        (else
          (bind (_path_2 _name_2) (`self.Set Feature Image Path` _index (`self.SolutionNo`)))
          (`self.ExportRender` _path_2 _name_2))))
    (:`Completed`
      (bind _thresholdcount (`self.GetThresholdNum`))
      (`self.StopMovement`)
      (bind _returnvalue_4 (`self.SendData` (`self.Connection ID`) (`self.Concat_BytesBytes` (`self.Conv_IntToBytes` (`|GetArrayItem` _thresholdcount)) (`self.Conv_StringToBytes` ",") (`self.Conv_IntToBytes` (`|GetArrayItem` _thresholdcount 1)))))
      (`KismetSystemLibrary.PrintString` "Sent" _returnvalue_4))))

(fn `CopyImageToPath`
  (params (SolutionNum :type Integer) (Index :type Integer) (TrainIndex :type Integer))
  (bind _returnvalue (`GameplayStatics.GetActorOfClass` "/Script/ProceduralGeneration.ProceduralRoom"))
  (`ProceduralRoom.CopyImage` _returnvalue SolutionNum Index TrainIndex))

(fn `ExportRender`
  (params (Path :type String) (Name :type String))
  (`KismetRenderingLibrary.ExportRenderTarget` "/Game/CharacterView.CharacterView" Path Name))

(fn `GetBoundingBox`
  (params (`Folder Num` :type Integer) (Idx :type Integer) (ResX :type Integer) (ResY :type Integer))
  (returns (IfBoundingBox :type Boolean))
  (bind _returnvalue (`GameplayStatics.GetActorOfClass` "/Script/ProceduralGeneration.ProceduralRoom"))
  (bind _returnvalue_2 (`ProceduralRoom.GetBoundingBox` _returnvalue `Folder Num` Idx ResX ResY))
  (return _returnvalue_2))

(fn `GetThresholdDetectionAcc`
  (returns (Accuracy :type "Array of Float (double-precision)"))
  (bind _returnvalue (`GameplayStatics.GetActorOfClass` "/Game/BluePrint/CharacterBP.CharacterBP_C"))
  (bind _returnvalue_2 (`ProceduralGenerationCharacter.ThresholdDetectionAccuracy` _returnvalue))
  (return _returnvalue_2))

(fn `GetThresholdNum`
  (returns (ThresholdCount :type "Array of Integer"))
  (bind _returnvalue (`GameplayStatics.GetActorOfClass` "/Game/BluePrint/CharacterBP.CharacterBP_C"))
  (bind _returnvalue_2 (`ProceduralGenerationCharacter.GetThresholdCount` _returnvalue))
  (return _returnvalue_2))

(fn `ResetThresholdCount`
  (bind _returnvalue (`GameplayStatics.GetActorOfClass` "/Game/BluePrint/CharacterBP.CharacterBP_C"))
  (`ProceduralGenerationCharacter.ResetThresholdCount` _returnvalue))

(fn `ResumeMovement`
  (bind _returnvalue (`GameplayStatics.GetActorOfClass` "/Game/BluePrint/CharacterBP.CharacterBP_C"))
  (`/Game/BluePrint/CharacterBP.ActivateCharacter` _returnvalue))

(fn `ResumeToTargets`
  (bind _returnvalue (`GameplayStatics.GetActorOfClass` "/Script/ProceduralGeneration.AutoAgent"))
  (`AutoAgent.ResetMovingTarget` _returnvalue))

(fn `Set Feature Image Path`
  (params (index :type Integer) (`folder num` :type Integer))
  (returns (Path :type String) (Name :type String))
  (bind _returnvalue (`GameplayStatics.GetActorOfClass` "/Game/BluePrint/CharacterBP.CharacterBP_C"))
  (bind _returnvalue_2 (`ProceduralGenerationCharacter.GetFeatureImgPath` _returnvalue index `folder num`))
  (return (`|GetArrayItem` _returnvalue_2) (`|GetArrayItem` _returnvalue_2 1)))

(fn `Set Focal Length`
  (params (`Focal Length` :type "Float (double-precision)"))
  (bind _returnvalue (`GameplayStatics.GetActorOfClass` "/Game/BluePrint/CharacterBP.CharacterBP_C"))
  (`/Game/BluePrint/CharacterBP.Set FL` _returnvalue `Focal Length`))

(fn `Set Orientation`
  (params (Pitch :type "Float (double-precision)"))
  (bind _returnvalue (`GameplayStatics.GetActorOfClass` "/Game/BluePrint/CharacterBP.CharacterBP_C"))
  (`ProceduralGenerationCharacter.ChangeOrientation` _returnvalue Pitch))

(fn `Set Resolution`
  (params (X :type Integer) (Y :type Integer))
  (`GameplayStatics.GetActorOfClass` "/Game/BluePrint/CharacterBP.CharacterBP_C"))

(fn `Set Sensor Size`
  (params (Width :type "Float (double-precision)") (Height :type "Float (double-precision)"))
  (bind _returnvalue (`GameplayStatics.GetActorOfClass` "/Game/BluePrint/CharacterBP.CharacterBP_C"))
  (`ProceduralGenerationCharacter.ChangeSensorSize` _returnvalue Width Height))

(fn `Set Train Image Path`
  (params (Index :type Integer) (`Folder Num` :type Integer))
  (returns (Path :type String) (Name :type String))
  (bind _returnvalue (`GameplayStatics.GetActorOfClass` "/Game/BluePrint/CharacterBP.CharacterBP_C"))
  (bind _returnvalue_2 (`ProceduralGenerationCharacter.GetTrainImgPath` _returnvalue Index `Folder Num`))
  (return (`|GetArrayItem` _returnvalue_2) (`|GetArrayItem` _returnvalue_2 1)))

(fn `SetResolution`
  (params (`Res X` :type Integer))
  (bind _returnvalue (`GameplayStatics.GetActorOfClass` "/Game/BluePrint/CharacterBP.CharacterBP_C"))
  (`/Game/BluePrint/CharacterBP.Set ResX` _returnvalue `Res X`))

(fn `StopMovement`
  (bind _returnvalue (`GameplayStatics.GetActorOfClass` "/Game/BluePrint/CharacterBP.CharacterBP_C"))
  (`/Game/BluePrint/CharacterBP.Deactivate Character` _returnvalue))

(fn `UserConstructionScript`)